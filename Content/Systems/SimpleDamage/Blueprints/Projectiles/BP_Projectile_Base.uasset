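; Base projectile actor for the SimpleDamage system that flies straight or homes on a Target.
; The construction script applies Speed and Gravity to ProjectileMovement and, given a valid Target, configures homing on its root component.
; BeginPlay ignores the owner for collision and aims the initial velocity at any Target.
; On hit, it fires the OnProjectileImpact dispatcher, spawns impact effect and sound, then destroys itself, leaving damage to listeners.
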(event `self.ReceiveBeginPlay`
  ;[1 1 0 0.5] OnBegin / Spawn In and determine if staright shot or lock top target
  (`PrimitiveComponent.IgnoreActorWhenMoving` (`self.BoxCollision`) (`self.GetOwner`) true)
  (`self.Target`
    (:`then`
      (`self.CE_RotateToTarget`))
    (:`else`)))

(event `CE_RotateToTarget`
  ;[1 1 0 0.5] CE_RotateToTarget
  (set `MovementComponent.Velocity` (* (`KismetMathLibrary.GetDirectionUnitVector` (`self.K2_GetActorLocation`) (`self.K2_GetActorLocation` (`self.Target`))) (`self.Speed`)) (`self.ProjectileMovement`)))

(event `self.BoxCollision.OnComponentHit`
  (params (HitComponent :type "PrimitiveComponent Object Reference") (OtherActor :type "Actor Object Reference") (OtherComp :type "PrimitiveComponent Object Reference") (NormalImpulse :type "Vector Structure") (Hit :type "HitResult Structure (by ref)"))
  (bind (_bblockinghit _binitialoverlap _time _distance _location) (`GameplayStatics.BreakHitResult` Hit))
  ;[1 1 0 0.5] Call OnProjectileImpact when Hit another Actor / Play Particle / Play Sound
  (`self.OnProjectileImpact` OtherActor Hit)
  (`GameplayStatics.SpawnEmitterAtLocation` (`self.ImpactEffect`) _location)
  (`GameplayStatics.PlaySoundAtLocation` (`self.ImpactSound`) _location (struct) 1.0 1.0 0.0 null null null null)
  (`self.K2_DestroyActor`))

(fn `UserConstructionScript`
  (bind _projectilemovement (`self.ProjectileMovement`))
  (set `ProjectileMovementComponent.InitialSpeed` (`self.Speed`) _projectilemovement)
  (set `ProjectileMovementComponent.MaxSpeed` (`self.Speed`) _projectilemovement)
  (set `ProjectileMovementComponent.ProjectileGravityScale` (`self.Gravity`) _projectilemovement)
  (`self.Target`
    (:`then`
      (set `ProjectileMovementComponent.bIsHomingProjectile` (`self.IsHoming?`) _projectilemovement)
      (set `ProjectileMovementComponent.HomingTargetComponent` (`Actor.RootComponent` (`self.Target`)) _projectilemovement))
    (:`else`)))