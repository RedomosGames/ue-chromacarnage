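; BP_Door is a procedural dungeon door that moves vertically in response to room events.
; On BeginPlay it binds to the player-entered-room and player-cleared-room events on GS_Game.
; Clearing a room plays the MoveDoor timeline to raise the mesh on Z, and entering a room reverses it.
; Box overlap only turns the mesh material green and does not move the door.
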(event `self.ReceiveBeginPlay`
  ;[0 1 0 0.5] Begin Play
  (bind _asgs_game (cast `/Game/ChromaCarnage/Default/GS_Game` (`GameplayStatics.GetGameState`)))
  (add `/Game/ChromaCarnage/Default/GS_Game.OnPlayerEnteredRoom` _asgs_game (`|CreateDelegate` :!event `B_OnPlayerEnteredRoom`))
  (add `/Game/ChromaCarnage/Default/GS_Game.OnPlayerClearedRoom` _asgs_game (`|CreateDelegate` :!event `B_OnPlayerClearedRoom`)))

(event `self.Box.OnComponentBeginOverlap`
  (params (OverlappedComponent :type "PrimitiveComponent Object Reference") (OtherActor :type "Actor Object Reference") (OtherComp :type "PrimitiveComponent Object Reference") (OtherBodyIndex :type Integer) (bFromSweep :type Boolean) (SweepResult :type "HitResult Structure (by ref)"))
  ;[0 1 0 0.5] Open/Close door
  (`PrimitiveComponent.SetMaterial` (`self.StaticMesh`) 0 "/AnimationSharing/AnimSharingGreen.AnimSharingGreen"))

(event `B_OnPlayerClearedRoom`
  ;[0 1 0 0.5] Open/Close door
  (bind (_direction _newtrack_0) (`Timeline|MoveDoor` :!label _label)
    (:`Update`
      (`SceneComponent.K2_SetRelativeLocation` (`self.StaticMesh`) (`KismetMathLibrary.MakeVector` 0.0 0.0 (`KismetMathLibrary.Lerp` 210.0 520.0 _newtrack_0)) false false))))

(event `B_OnPlayerEnteredRoom`
  ;[0 1 0 0.5] Open/Close door
  (goto _label :!via `Reverse`))

(event `self.Box.OnComponentEndOverlap`
  (params (OverlappedComponent :type "PrimitiveComponent Object Reference") (OtherActor :type "Actor Object Reference") (OtherComp :type "PrimitiveComponent Object Reference") (OtherBodyIndex :type Integer))
  ;[0 1 0 0.5] Open/Close door
)

(fn `UserConstructionScript`)