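; An acid mist area actor that applies an acid effect to pawns around its location.
; On BeginPlay it starts a looping timer and runs a debug-drawn multi-sphere trace, sending IFAcidEffectMessage with UniqueDamage to each hit actor.
; Each timer tick decrements LoopTime and repeats the trace while LoopTime is zero or below; otherwise it clears the timer and destroys the actor.
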(event `self.ReceiveBeginPlay`
  (bind _returnvalue (`self.K2_GetActorLocation`))
  (bind _returnvalue_2 (`KismetSystemLibrary.K2_SetTimerDelegate` (delegate `T_AcidMist`) 0.25 true))
  (bind (_outhits _returnvalue_3) (`KismetSystemLibrary.SphereTraceMultiForObjects` :`Start` _returnvalue :`End` _returnvalue :`Radius` 300.0 :`ObjectTypes` (`|MakeArray` "ObjectTypeQuery3" :!type "EObjectTypeQuery Enum") :`DrawDebugType` "ForDuration" :!label _label))
  (if _returnvalue_3
    (for _array_element _outhits
      (message `/Game/Systems/Guns/Blueprints/Interfaces/BPI_GunEffects.IF_AcidEffect` (`.HitActor` (`GameplayStatics.BreakHitResult` _array_element)) (`self.UniqueDamage`)))))

(event `T_AcidMist`
  (if (<= (`self.LoopTime`) 0)
    (`/Engine/EditorBlueprintResources/StandardMacros.DecrementInt` (`self.LoopTime`)
      (:`  `
        (goto _label)))
    (else
      (`KismetSystemLibrary.K2_ClearAndInvalidateTimerHandle` (stale `self.ReceiveBeginPlay` _returnvalue_2))
      (`self.K2_DestroyActor`))))

(fn `UserConstructionScript`)