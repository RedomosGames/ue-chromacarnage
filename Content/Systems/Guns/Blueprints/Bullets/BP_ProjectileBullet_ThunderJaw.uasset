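; BP_ProjectileBullet_ThunderJaw is a gun projectile that applies a shock effect on impact and spreads it to a nearby target.
; On hit it runs the parent logic, then sends the shock interface message with UniqueDamage to the struck actor.
; FShockTrace then searches a radius around the hit, passing that actor as HitEnemy, and shocks the actor it returns.
; Each hit decrements BounceAmount, and the bullet destroys itself once none remain.
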(event `self.ReceiveBeginPlay`
  (`parent.ReceiveBeginPlay`))

(event `self.ReceiveHit`
  (params (MyComp :type "PrimitiveComponent Object Reference") (Other :type "Actor Object Reference") (OtherComp :type "PrimitiveComponent Object Reference") (bSelfMoved :type Boolean) (HitLocation :type "Vector Structure") (HitNormal :type "Vector Structure") (NormalImpulse :type "Vector Structure") (Hit :type "HitResult Structure (by ref)"))
  (bind _bounceamount (`self.BounceAmount`))
  (`parent.ReceiveHit` MyComp Other OtherComp bSelfMoved HitLocation HitNormal NormalImpulse Hit)
  (message `/Game/Systems/Guns/Blueprints/Interfaces/BPI_GunEffects.IF_ShockEffect` Other (`self.UniqueDamage`))
  (bind _outhit (`self.F_ShockTrace` 250.0 Other))
  (message `/Game/Systems/Guns/Blueprints/Interfaces/BPI_GunEffects.IF_ShockEffect` (`.HitActor` (`GameplayStatics.BreakHitResult` _outhit)) (`self.UniqueDamage`))
  (`/Engine/EditorBlueprintResources/StandardMacros.DecrementInt` _bounceamount
    (:`  `
      (if (<= _bounceamount 0)
        (`self.K2_DestroyActor`)))))

(fn `UserConstructionScript`
  (`parent.UserConstructionScript`))