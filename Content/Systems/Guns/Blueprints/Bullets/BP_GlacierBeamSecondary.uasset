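; Secondary-fire projectile for the Glacier Beam gun that leaves a blizzard slowing nearby pawns after impact.
; BeginPlay sets the Niagara tracer, and the first Hit event spawns impact VFX and starts a looping timer.
; Each tick sphere-traces around the actor and sends a slow-down interface message, until LoopAmount runs out and the actor destroys itself.
; Explosive and shock trace helper functions are defined but not called here.
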(event `self.ReceiveBeginPlay`
  ;[0 1 0 0.5] Set Niagara VFX
  (`NiagaraComponent.SetAsset` (`self.TracerVisuals`) (`self.TracerVFX`) true))

(event `self.ReceiveHit`
  (params (MyComp :type "PrimitiveComponent Object Reference") (Other :type "Actor Object Reference") (OtherComp :type "PrimitiveComponent Object Reference") (bSelfMoved :type Boolean) (HitLocation :type "Vector Structure") (HitNormal :type "Vector Structure") (NormalImpulse :type "Vector Structure") (Hit :type "HitResult Structure (by ref)"))
  ;[0 1 0 0.5] Activate Impact VFX
  (`/Engine/EditorBlueprintResources/StandardMacros.DoOnce` false
    (:`Completed`
      (`KismetSystemLibrary.PrintString` "Impact")
      (`NiagaraFunctionLibrary.SpawnSystemAtLocation` (`self.ImpactVFX`) HitLocation)
      (`KismetSystemLibrary.K2_SetTimerDelegate` (delegate `T_BlizzardEffect`) 0.5 true))))

(event `T_BlizzardEffect`
  (bind _returnvalue (`self.K2_GetActorLocation`))
  ;[0 1 0 0.5] Activate Impact VFX
  (if (> (`self.LoopAmount`) 0)
    (`/Engine/EditorBlueprintResources/StandardMacros.DecrementInt` (`self.LoopAmount`)
      (:`  `
        (bind (_outhits _returnvalue_2) (`KismetSystemLibrary.SphereTraceMultiForObjects` :`Start` _returnvalue :`End` _returnvalue :`Radius` 1000.0 :`ObjectTypes` (`|MakeArray` "ObjectTypeQuery3" :!type "EObjectTypeQuery Enum") :`DrawDebugType` "ForDuration"))
        (if _returnvalue_2
          (for _array_element _outhits
            (message `/Game/Systems/Guns/Blueprints/Interfaces/BPI_GunEffects.IF_SlowDown` (`.HitActor` (`GameplayStatics.BreakHitResult` _array_element)))))))
    (else
      (`self.K2_DestroyActor`))))

(fn `F_ExplosiveTrace`
  (params (Radius :type "Float (single-precision)"))
  (returns (OutHits :type "Array of HitResult Structure"))
  (bind _returnvalue (`self.K2_GetActorLocation`))
  (bind _outhits (`KismetSystemLibrary.SphereTraceMultiForObjects` :`Start` _returnvalue :`End` _returnvalue :`Radius` Radius :`ObjectTypes` (`|MakeArray` "ObjectTypeQuery3" :!type "EObjectTypeQuery Enum") :`DrawDebugType` "ForDuration" :`DrawTime` 1.0))
  (return _outhits))

(fn `F_ShockTrace`
  (params (Radius :type "Float (single-precision)") (HitEnemy :type "Actor Object Reference"))
  (returns (OutHit :type "HitResult Structure"))
  (bind _returnvalue (`self.K2_GetActorLocation`))
  (bind _outhit (`KismetSystemLibrary.SphereTraceSingleForObjects` _returnvalue _returnvalue Radius (`|MakeArray` "ObjectTypeQuery3" :!type "EObjectTypeQuery Enum") false (`|MakeArray` HitEnemy)))
  (return _outhit))

(fn `UserConstructionScript`)