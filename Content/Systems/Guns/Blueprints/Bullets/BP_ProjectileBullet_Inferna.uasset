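; Inferna gun bullet projectile that can home in on a target and deals explosive area damage on impact.
; On BeginPlay, a valid HomingTarget turns on ProjectileMovement homing toward that actor's root component with strong acceleration.
; The first hit, gated by DoOnce, runs the parent hit logic, applies damage to every actor found by an explosive trace, then destroys the bullet.
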(event `self.ReceiveBeginPlay`
  (bind _projectilemovement (`self.ProjectileMovement`))
  (`parent.ReceiveBeginPlay`)
  (bind _homingtarget (`self.HomingTarget`)
    (:`then`
      (set `ProjectileMovementComponent.bIsHomingProjectile` true _projectilemovement)
      (set `ProjectileMovementComponent.HomingTargetComponent` (`Actor.RootComponent` _homingtarget) _projectilemovement)
      (set `ProjectileMovementComponent.HomingAccelerationMagnitude` 10000.0 _projectilemovement))
    (:`else`)))

(event `self.ReceiveHit`
  (params (MyComp :type "PrimitiveComponent Object Reference") (Other :type "Actor Object Reference") (OtherComp :type "PrimitiveComponent Object Reference") (bSelfMoved :type Boolean) (HitLocation :type "Vector Structure") (HitNormal :type "Vector Structure") (NormalImpulse :type "Vector Structure") (Hit :type "HitResult Structure (by ref)"))
  (`/Engine/EditorBlueprintResources/StandardMacros.DoOnce` false
    (:`Completed`
      (`parent.ReceiveHit` MyComp Other OtherComp bSelfMoved HitLocation HitNormal NormalImpulse Hit)
      (bind _outhits (`self.F_ExplosiveTrace` 200.0))
      (for _array_element _outhits
        (`self.CE_ApplyDamage` (`.HitActor` (`GameplayStatics.BreakHitResult` _array_element))))
      (`self.K2_DestroyActor`))))

(fn `UserConstructionScript`
  (`parent.UserConstructionScript`))