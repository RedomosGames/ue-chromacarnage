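; BP_ProjectileBullet_CryoLance is a gun projectile that damages and slows what it hits.
; On collision overlap it spawns an impact VFX at the sweep location, then sends damage and slow-down interface messages to the other actor.
; The projectile destroys itself only on a Hit event, so overlaps alone do not stop it.
; The overlap handler also prints a debug string.
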(event `self.ReceiveBeginPlay`
  (`parent.ReceiveBeginPlay`))

(event `self.ReceiveHit`
  (params (MyComp :type "PrimitiveComponent Object Reference") (Other :type "Actor Object Reference") (OtherComp :type "PrimitiveComponent Object Reference") (bSelfMoved :type Boolean) (HitLocation :type "Vector Structure") (HitNormal :type "Vector Structure") (NormalImpulse :type "Vector Structure") (Hit :type "HitResult Structure (by ref)"))
  (`self.K2_DestroyActor`))

(event `self.Collision.OnComponentBeginOverlap`
  (params (OverlappedComponent :type "PrimitiveComponent Object Reference") (OtherActor :type "Actor Object Reference") (OtherComp :type "PrimitiveComponent Object Reference") (OtherBodyIndex :type Integer) (bFromSweep :type Boolean) (SweepResult :type "HitResult Structure (by ref)"))
  (`KismetSystemLibrary.PrintString` "Overlap")
  (`NiagaraFunctionLibrary.SpawnSystemAtLocation` (`self.ImpactVFX`) (`.Location` (`GameplayStatics.BreakHitResult` SweepResult)))
  (message `/Game/Systems/SimpleDamage/Blueprints/Interfaces/BPI_Damagable.IF_TakeDamage` OtherActor (make `/Game/Systems/SimpleDamage/Blueprints/Data/S_DamageInfo` (`self.Damage`) "NewEnumerator2"))
  (message `/Game/Systems/Guns/Blueprints/Interfaces/BPI_GunEffects.IF_SlowDown` OtherActor))

(fn `UserConstructionScript`
  (`parent.UserConstructionScript`))