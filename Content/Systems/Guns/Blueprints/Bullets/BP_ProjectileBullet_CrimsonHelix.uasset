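; Projectile bullet for the Crimson Helix gun that sticks to what it hits and explodes after a short delay.
; On hit it runs the parent bullet logic, disables collision and attaches itself to the struck actor.
; After a one-second fuse, an explosive trace gathers nearby actors, sends each UniqueDamage through a damage interface message, then the bullet destroys itself.
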(event `self.ReceiveBeginPlay`
  (`parent.ReceiveBeginPlay`))

(event `self.ReceiveHit`
  (params (MyComp :type "PrimitiveComponent Object Reference") (Other :type "Actor Object Reference") (OtherComp :type "PrimitiveComponent Object Reference") (bSelfMoved :type Boolean) (HitLocation :type "Vector Structure") (HitNormal :type "Vector Structure") (NormalImpulse :type "Vector Structure") (Hit :type "HitResult Structure (by ref)"))
  (`parent.ReceiveHit` MyComp Other OtherComp bSelfMoved HitLocation HitNormal NormalImpulse Hit)
  (`PrimitiveComponent.SetCollisionEnabled` (`self.Collision`) "NoCollision")
  (`self.K2_AttachToActor` Other "None" "KeepWorld" "KeepRelative" "KeepWorld")
  (`KismetSystemLibrary.Delay` 1.0)
  (bind _outhits (`self.F_ExplosiveTrace` 300.0))
  (for _array_element _outhits
    (message `/Game/Systems/SimpleDamage/Blueprints/Interfaces/BPI_Damagable.IF_TakeDamage` (`.HitActor` (`GameplayStatics.BreakHitResult` _array_element)) (make `/Game/Systems/SimpleDamage/Blueprints/Data/S_DamageInfo` (`self.UniqueDamage`) "NewEnumerator3")))
  (`self.K2_DestroyActor`))

(fn `UserConstructionScript`
  (`parent.UserConstructionScript`))