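; BP_ProjectileBullet is a projectile bullet actor for the gun system that damages what it hits.
; On BeginPlay it assigns its tracer effect to the TracerVisuals Niagara component.
; On Hit it prints a debug string, spawns the impact effect at the hit location and sends damage info to the other actor through an interface message.
; It then destroys itself.
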(event `self.ReceiveBeginPlay`
  ;[0 1 0 0.5] Set Niagara VFX
  (`NiagaraComponent.SetAsset` (`self.TracerVisuals`) (`self.TracerVFX`) true))

(event `self.ReceiveHit`
  (params (MyComp :type "PrimitiveComponent Object Reference") (Other :type "Actor Object Reference") (OtherComp :type "PrimitiveComponent Object Reference") (bSelfMoved :type Boolean) (HitLocation :type "Vector Structure") (HitNormal :type "Vector Structure") (NormalImpulse :type "Vector Structure") (Hit :type "HitResult Structure (by ref)"))
  ;[0 1 0 0.5] Activate Impact VFX / Apply Damage / Destroy
  (`KismetSystemLibrary.PrintString` "Impact")
  (`NiagaraFunctionLibrary.SpawnSystemAtLocation` (`self.ImpactVFX`) HitLocation)
  (message `/Game/Systems/SimpleDamage/Blueprints/Interfaces/BPI_Damagable.IF_TakeDamage` Other (make `/Game/Systems/SimpleDamage/Blueprints/Data/S_DamageInfo` :`Amount` (`self.Damage`)))
  (`self.K2_DestroyActor`))

(fn `UserConstructionScript`)