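; BP_Enemy_Flying is a flying enemy Blueprint that extends its parent's attack interface event with a two-stage ranged attack.
; It plays a buster-ready montage with a sound, and a montage notify then triggers the fire montage.
; Firing clears AI focus and spawns BP_FlyingRange at the AttackSpawn point with a second sound.
; The fire montage calls IFAttackEnd on completion or interruption.
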(event `self.IF_Attack`
  (params (AttackTarget :type "Actor Object Reference") (IsMeleeAttack :type Boolean) (BossAttack :type "/Game/ChromaCarnage/Blueprints/Enemies/AI/E_BossAttacks Enum" :default "NewEnumerator0"))
  (`parent.IF_Attack` AttackTarget IsMeleeAttack BossAttack)
  (bind _notifyname (`|PlayMontage` (`self.Mesh`) "/Game/Robot02/Mesh/Animations/Combat/Robot02_Idle_BusterReady_Montage.Robot02_Idle_BusterReady_Montage")
    (:`then`
      (`GameplayStatics.PlaySoundAtLocation` "/Engine/VREditor/Sounds/UI/Teleport_Mode_Entered.Teleport_Mode_Entered" (`self.K2_GetActorLocation`) (struct) 1.0 1.0 0.0 null null null null))
    (:`OnNotifyBegin`
      (switch `name` _notifyname
        (:`Attack`
          (`|PlayMontage` (`self.Mesh`) "/Game/Robot02/Mesh/Animations/Combat/Robot02_FireBuster_Montage.Robot02_FireBuster_Montage"
            (:`then`
              (`AIController.K2_ClearFocus` (`AIBlueprintHelperLibrary.GetAIController` self))
              (`|SpawnActorFromClass` "/Game/ChromaCarnage/Blueprints/Enemies/AI/BP_FlyingRange.BP_FlyingRange_C" (`KismetMathLibrary.MakeTransform` (`SceneComponent.K2_GetComponentLocation` (`self.AttackSpawn`))) "Undefined" "MultiplyWithRoot" null null)
              (`GameplayStatics.PlaySoundAtLocation` "/Engine/VREditor/Sounds/UI/Foliage_Placed.Foliage_Placed" (`self.K2_GetActorLocation`) (struct) 1.0 1.0 0.0 null null null null))
            (:`OnCompleted`
              (`/Game/Systems/SimpleDamage/Blueprints/Interfaces/BPI_Damagable.IF_AttackEnd` AttackTarget :!label _label))
            (:`OnInterrupted`
              (goto _label))))))))

(fn `UserConstructionScript`
  (`parent.UserConstructionScript`))