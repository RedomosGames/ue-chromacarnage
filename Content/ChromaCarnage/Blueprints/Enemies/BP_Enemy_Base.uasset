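; BP_Enemy_Base is the base enemy character, with a health bar, movement speed by state, and launch-arc jumps to navlink destinations.
; Health and damage route through BPC_DamageSystem, with one-tick immunity against multi-trace hits, alongside slow, acid, shock and explosion-knockback effects.
; Attacks reserve tokens from their target and return them on completion or death.
; Death ragdolls the mesh, removes the enemy from GS_Game's tracking, then destroys it.
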(event `/Game/Systems/Guns/Blueprints/Interfaces/BPI_GunEffects.IF_SlowDown`
  (bind _charactermovement (`self.CharacterMovement`))
  (bind _charactermovement_2 (`self.CharacterMovement`))
  ;[0 1 0 0.5] Weapon Effects
  (if (not (`self.IsSlowedDown`))
    (set `self.IsSlowedDown` true)
    (set `CharacterMovementComponent.MaxWalkSpeed` (/ (`CharacterMovementComponent.MaxWalkSpeed` _charactermovement) 2.0) _charactermovement))
  (`KismetSystemLibrary.RetriggerableDelay` 5.0)
  (set `self.IsSlowedDown` false)
  (set `CharacterMovementComponent.MaxWalkSpeed` (* (`CharacterMovementComponent.MaxWalkSpeed` _charactermovement_2) 2.0) _charactermovement_2))

(event `self.ReceiveBeginPlay`
  ;[0 1 0 0.5] Begin Play
  (`|ExecutionSequence`
    (:`then_0`
      (bind _asgs_game (cast `/Game/ChromaCarnage/Default/GS_Game` (`GameplayStatics.GetGameState`)))
      (set `self.GsRef` _asgs_game)
      (bind _asai_enemy_base (cast `/Game/ChromaCarnage/Blueprints/Enemies/AI/AI_Enemy_Base` (`AIBlueprintHelperLibrary.GetAIController` self)))
      (set `self.AicRef` _asai_enemy_base))
    (:`then_1`
      (bind _returnvalue (`|CreateWidget` "/Game/Systems/SimpleDamage/Blueprints/Widget/WBP_HealthBar.WBP_HealthBar_C" null self))
      (`WidgetComponent.SetWidget` (`self.Healthbar`) _returnvalue))))

(event `/Game/Systems/Guns/Blueprints/Interfaces/BPI_GunEffects.IF_AcidEffect`
  (params (UniqueDamage :type "Float (double-precision)"))
  ;[0 1 0 0.5] Weapon Effects
  (set `self.AcidLoop` 5)
  (`KismetSystemLibrary.K2_ClearAndInvalidateTimerHandle` (stale _returnvalue))
  (bind _returnvalue (`KismetSystemLibrary.K2_SetTimerDelegate` (delegate `T_AppleDissolveDamage`) 1.0 true))
  (if (>= (`self.AcidLoop`) 1) :!label _label
    (`/Engine/EditorBlueprintResources/StandardMacros.DecrementInt` (`self.AcidLoop`)
      (:`  `
        (`self.IF_TakeDamage` (make `/Game/Systems/SimpleDamage/Blueprints/Data/S_DamageInfo` UniqueDamage))
        (`KismetSystemLibrary.PrintString` "Acid DMG")))
    (else
      (`KismetSystemLibrary.K2_ClearAndInvalidateTimerHandle` _returnvalue))))

(event `T_AppleDissolveDamage`
  ;[0 1 0 0.5] Weapon Effects
  (goto _label))

(event `/Game/Systems/SimpleDamage/Blueprints/Interfaces/BPI_Damagable.IF_ReturnAttackToken`
  (params (Amount :type Integer))
  ;[0 1 0 0.5] Attack Token Functionality
  (`/Game/Systems/SimpleDamage/Blueprints/Components/BPC_DamageSystem.F_ReturnAttackToken` (`self.BPC_DamageSystem`) Amount))

(event `/Game/Systems/SimpleDamage/Blueprints/Interfaces/BPI_Damagable.IF_StoreAttackTokens`
  (params (AttackTarget :type "Actor Object Reference") (Amount :type Integer))
  (bind (_value _returnvalue) (`BlueprintMapLibrary.Map_Find` (`self.ReservedAttackTokens`) AttackTarget))
  ;[0 1 0 0.5] Attack Token Functionality
  (`BlueprintMapLibrary.Map_Add` (`self.ReservedAttackTokens`) AttackTarget (`KismetMathLibrary.SelectInt` (+ Amount _value) Amount _returnvalue))
  (set `self.TokensUsedInCurretnAttack` 0))

(event `/Game/ChromaCarnage/Blueprints/Enemies/AI/BPI_Enemy.IF_JumpToDestination`
  (params (Destination :type "Vector Structure"))
  ;[0 1 0 0.5] Jump to NavLink Location
  (bind _outlaunchvelocity (`GameplayStatics.SuggestProjectileVelocity_CustomArc` (`self.K2_GetActorLocation`) (`KismetMathLibrary.MakeVector` (.x Destination) (.y Destination) (+ (.z Destination) 200.0))))
  (`self.LaunchCharacter` _outlaunchvelocity true true))

(event `/Game/Systems/Guns/Blueprints/Interfaces/BPI_GunEffects.IF_ShockEffect`
  (params (UniqueDamage :type "Float (double-precision)"))
  ;[0 1 0 0.5] Weapon Effects
  (`self.IF_TakeDamage` (make `/Game/Systems/SimpleDamage/Blueprints/Data/S_DamageInfo` UniqueDamage))
  (if (not (`self.IsShocked`))
    (set `self.IsShocked` true)
    (`CharacterMovementComponent.SetMovementMode` (`self.CharacterMovement`) "MOVE_None" 0))
  (`KismetSystemLibrary.RetriggerableDelay` 1.0)
  (set `self.IsShocked` false)
  (`CharacterMovementComponent.SetMovementMode` (`self.CharacterMovement`) "MOVE_Walking" 0))

(event `/Game/Systems/SimpleDamage/Blueprints/Interfaces/BPI_Damagable.IF_AttackEnd`
  (params (AttackTarget :type "Actor Object Reference"))
  (bind _tokensusedincurretnattack (`self.TokensUsedInCurretnAttack`))
  ;[0 1 0 0.5] Attack Token Functionality
  (message `/Game/Systems/SimpleDamage/Blueprints/Interfaces/BPI_Damagable.IF_ReturnAttackToken` AttackTarget _tokensusedincurretnattack)
  (`/Game/Systems/SimpleDamage/Blueprints/Interfaces/BPI_Damagable.IF_StoreAttackTokens` AttackTarget (* _tokensusedincurretnattack -1))
  (`self.OnAttackComplete`)
  (set `self.TokensUsedInCurretnAttack` 0))

(event `CE_ResetDamageImunituy`
  ;[0 1 0 0.5] Reset Damage Immunity for Multi Trace
  (`KismetSystemLibrary.DelayUntilNextTick`)
  (set `self.CanTakeDMG` true))

(event `/Game/Systems/Guns/Blueprints/Interfaces/BPI_GunEffects.IF_Explosion`
  (bind (_returnvalue_x _returnvalue_y _returnvalue_z) (`KismetMathLibrary.BreakVector` (* (`KismetMathLibrary.GetForwardVector` (`self.K2_GetActorRotation`)) -1500.0)))
  ;[0 1 0 0.5] Weapon Effects
  (`CharacterMovementComponent.SetMovementMode` (`self.CharacterMovement`) "MOVE_Flying" 0)
  (`self.LaunchCharacter` (`KismetMathLibrary.MakeVector` _returnvalue_x _returnvalue_y (+ _returnvalue_z 350.0)) true true)
  (`KismetSystemLibrary.RetriggerableDelay` 1.0)
  (`CharacterMovementComponent.SetMovementMode` (`self.CharacterMovement`) "MOVE_Walking" 0))

(event `self.BPC_DamageSystem.OnDeath`
  ;[0 1 0 0.5] On Death
  (if (`self.DoNormalDeath`)
    (`/Engine/EditorBlueprintResources/StandardMacros.DoOnce` false
      (:`Completed`
        (`PrimitiveComponent.SetSimulatePhysics` (`self.Mesh`) true)
        (`PrimitiveComponent.SetCollisionEnabled` (`self.Mesh`) "QueryAndPhysics")
        (`self.CE_RestoreInfo`)
        (`KismetSystemLibrary.Delay` 0.25)
        (`self.K2_DestroyActor`)))))

(event `CE_RestoreInfo`
  (bind _tokensusedincurretnattack (`self.TokensUsedInCurretnAttack`))
  ;[0 1 0 0.5] CE_RestoreInfo
  (message `/Game/Systems/SimpleDamage/Blueprints/Interfaces/BPI_Damagable.IF_ReturnAttackToken` (`GameplayStatics.GetPlayerCharacter` 0) _tokensusedincurretnattack)
  (`/Game/Systems/SimpleDamage/Blueprints/Interfaces/BPI_Damagable.IF_StoreAttackTokens` null (* _tokensusedincurretnattack -1))
  (`/Game/ChromaCarnage/Default/GS_Game.CE_RemoveEnemy` (`self.GsRef`)))

(fn `F_SetMovementSpeed`
  (params (EnemyState :type "/Game/ChromaCarnage/Blueprints/Enemies/AI/E_EnemyState Enum" :default "NewEnumerator0"))
  (switch `/Game/ChromaCarnage/Blueprints/Enemies/AI/E_EnemyState` EnemyState
    (:`NewEnumerator1`
      (set `CharacterMovementComponent.MaxWalkSpeed` (`self.WaitingSpeed`) (`self.CharacterMovement`)))
    (:`NewEnumerator2`
      (set `CharacterMovementComponent.MaxWalkSpeed` (`self.AttackingSpeed`) (`self.CharacterMovement`)))
    (:`NewEnumerator4`
      (set `CharacterMovementComponent.MaxWalkSpeed` 0.0 (`self.CharacterMovement`)))))

(fn `IF_AttackStart`
  (params (AttackTarget :type "Actor Object Reference") (TokenNeeded :type Integer))
  (returns (Success :type Boolean))
  (bind _success (message `/Game/Systems/SimpleDamage/Blueprints/Interfaces/BPI_Damagable.IF_ReserveAttackToken` AttackTarget TokenNeeded))
  (if _success
    (`/Game/Systems/SimpleDamage/Blueprints/Interfaces/BPI_Damagable.IF_StoreAttackTokens` AttackTarget TokenNeeded)
    (set `self.TokensUsedInCurretnAttack` TokenNeeded)
    (return true)
    (else
      (return false))))

(fn `IF_GetCurrentHealth`
  (returns (Health :type "Float (double-precision)"))
  (return (`/Game/Systems/SimpleDamage/Blueprints/Components/BPC_DamageSystem.Health` (`self.BPC_DamageSystem`))))

(fn `IF_GetMaxHealth`
  (returns (MaxHealth :type "Float (double-precision)"))
  (return (`/Game/Systems/SimpleDamage/Blueprints/Components/BPC_DamageSystem.MaxHealth` (`self.BPC_DamageSystem`))))

(fn `IF_Heal`
  (params (Amount :type "Float (double-precision)"))
  (returns (NewHealth :type "Float (double-precision)"))
  (bind _newhealth (`/Game/Systems/SimpleDamage/Blueprints/Components/BPC_DamageSystem.F_Heal` (`self.BPC_DamageSystem`) Amount))
  (return _newhealth))

(fn `IF_ReserveAttackToken`
  (params (Amount :type Integer))
  (returns (Success :type Boolean))
  (bind _success (`/Game/Systems/SimpleDamage/Blueprints/Components/BPC_DamageSystem.F_ReserveAttackToken` (`self.BPC_DamageSystem`) Amount))
  (return _success))

(fn `IF_TakeDamage`
  (params (DamageInfo :type "/Game/Systems/SimpleDamage/Blueprints/Data/S_DamageInfo Structure"))
  (returns (`WasDamaged?` :type Boolean))
  (if (`self.CanTakeDMG`)
    (set `self.CanTakeDMG` false)
    (`/Game/Systems/SimpleDamage/Blueprints/Components/BPC_DamageSystem.F_TakeDamage` (`self.BPC_DamageSystem`) DamageInfo)
    (`/Game/ChromaCarnage/Default/GS_Game.OnEnemyDamaged` (`self.GsRef`))
    (`KismetSystemLibrary.PrintString` "TOOK DMG")
    (`self.CE_ResetDamageImunituy`)
    (return false)))

(fn `UserConstructionScript`)