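; Brute enemy Blueprint that extends its parent's attack interface with montage-driven melee and ranged attacks.
; Melee launches the Brute along a calculated arc at the player, then a montage notify triggers a sphere-trace damage burst with lightning effects.
; Ranged plays a half-speed montage whose notify spawns three staggered BP_BruteRange actors, aimed below the player's location.
; Both attacks signal attack end when their montage completes or is interrupted.
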(event `self.IF_Attack`
  (params (AttackTarget :type "Actor Object Reference") (IsMeleeAttack :type Boolean) (BossAttack :type "/Game/ChromaCarnage/Blueprints/Enemies/AI/E_BossAttacks Enum" :default "NewEnumerator0"))
  (bind _returnvalue (`self.K2_GetActorLocation`))
  (`parent.IF_Attack` AttackTarget IsMeleeAttack "NewEnumerator0")
  (if IsMeleeAttack
    (bind _notifyname (`|PlayMontage` (`self.Mesh`) "/Game/Imports/Animations/BruteMelee_Montage.BruteMelee_Montage")
      (:`then`
        (`GameplayStatics.PlaySoundAtLocation` "/Engine/EditorSounds/GamePreview/PossessPlayer_Cue.PossessPlayer_Cue" (`self.K2_GetActorLocation`) (struct) 1.0 1.0 0.0 null null null null)
        (bind _outlaunchvelocity (`GameplayStatics.SuggestProjectileVelocity_CustomArc` (`self.K2_GetActorLocation`) (`self.K2_GetActorLocation` (`GameplayStatics.GetPlayerCharacter` 0))))
        (`self.LaunchCharacter` _outlaunchvelocity true true))
      (:`OnCompleted`
        (`/Game/Systems/SimpleDamage/Blueprints/Interfaces/BPI_Damagable.IF_AttackEnd` AttackTarget :!label _label))
      (:`OnInterrupted`
        (goto _label))
      (:`OnNotifyBegin`
        (switch `name` _notifyname
          (:`Attack`
            (bind (_outhit _returnvalue_2) (`KismetSystemLibrary.SphereTraceSingleForObjects` :`Start` _returnvalue :`End` _returnvalue :`Radius` 500.0 :`ObjectTypes` (`|MakeArray` "ObjectTypeQuery9" :!type "EObjectTypeQuery Enum") :`DrawDebugType` "ForDuration"))
            (if _returnvalue_2
              (message `/Game/Systems/SimpleDamage/Blueprints/Interfaces/BPI_Damagable.IF_TakeDamage` (`.HitActor` (`GameplayStatics.BreakHitResult` _outhit)) (make `/Game/Systems/SimpleDamage/Blueprints/Data/S_DamageInfo` :`Amount` 5.0)))
            (`GameplayStatics.SpawnEmitterAtLocation` "/Game/Systems/SimpleDamage/FXVarietyPack/Particles/P_ky_lightning2.P_ky_lightning2" (`self.K2_GetActorLocation`))
            (`GameplayStatics.PlaySoundAtLocation` "/Engine/VREditor/Sounds/VR_ungrab.VR_ungrab" (`self.K2_GetActorLocation`) (struct) 1.0 1.0 0.0 null null null null)))))
    (else
      (bind _notifyname_2 (`|PlayMontage` (`self.Mesh`) "/Game/Imports/Animations/BruteRange_Montage.BruteRange_Montage" 0.5)
        (:`then`
          (`GameplayStatics.SpawnEmitterAtLocation` "/Game/Systems/SimpleDamage/FXVarietyPack/Particles/P_ky_lightning1.P_ky_lightning1" (`self.K2_GetActorLocation`)))
        (:`OnCompleted`
          (`/Game/Systems/SimpleDamage/Blueprints/Interfaces/BPI_Damagable.IF_AttackEnd` null :!label _label_2))
        (:`OnInterrupted`
          (goto _label_2))
        (:`OnNotifyBegin`
          (switch `name` _notifyname_2
            (:`Range Attack`
              (`self.CE_SpawnRangeAttack`)
              (`KismetSystemLibrary.Delay` 0.8)
              (`self.CE_SpawnRangeAttack`)
              (`KismetSystemLibrary.Delay` 0.8)
              (`self.CE_SpawnRangeAttack`))))))))

(event `CE_SpawnRangeAttack`
  (bind (_returnvalue_x _returnvalue_y _returnvalue_z) (`KismetMathLibrary.BreakVector` (`self.K2_GetActorLocation` (`GameplayStatics.GetPlayerCharacter` 0))))
  (`|SpawnActorFromClass` "/Game/ChromaCarnage/Blueprints/Enemies/AI/BP_BruteRange.BP_BruteRange_C" (`KismetMathLibrary.MakeTransform` (`SceneComponent.K2_GetComponentLocation` (`self.RangeSpawn`)) (`KismetMathLibrary.FindLookAtRotation` (`self.K2_GetActorLocation`) (`KismetMathLibrary.MakeVector` _returnvalue_x _returnvalue_y (- _returnvalue_z 225.0)))) "Undefined" "MultiplyWithRoot" null null)
  (`GameplayStatics.PlaySoundAtLocation` "/Engine/VREditor/Sounds/UI/Object_Snaps_To_Another_Actor.Object_Snaps_To_Another_Actor" (`self.K2_GetActorLocation`) (struct) 1.0 1.0 0.0 null null null null))

(fn `UserConstructionScript`
  (`parent.UserConstructionScript`))