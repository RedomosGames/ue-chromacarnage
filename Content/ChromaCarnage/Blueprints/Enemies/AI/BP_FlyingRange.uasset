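; Explosive projectile, apparently for a flying ranged enemy, that lobs itself at the player.
; On spawn it computes a custom-arc launch velocity to the player's current position, with no later homing.
; On hit it sphere-traces around itself, sends damage through an interface message to the first actor found, plays explosion effects and sound, then destroys itself.
; Debug print and trace drawing remain enabled.
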(event `self.ReceiveBeginPlay`
  (bind _outlaunchvelocity (`GameplayStatics.SuggestProjectileVelocity_CustomArc` (`self.K2_GetActorLocation`) (`self.K2_GetActorLocation` (`GameplayStatics.GetPlayerCharacter` 0))))
  (set `MovementComponent.Velocity` _outlaunchvelocity (`self.ProjectileMovement`)))

(event `self.Projectile Collision.OnComponentHit`
  (params (HitComponent :type "PrimitiveComponent Object Reference") (OtherActor :type "Actor Object Reference") (OtherComp :type "PrimitiveComponent Object Reference") (NormalImpulse :type "Vector Structure") (Hit :type "HitResult Structure (by ref)"))
  (bind _returnvalue (`self.K2_GetActorLocation`))
  (`KismetSystemLibrary.PrintString` "Flying RANGE IMAPCT")
  (bind (_outhit _returnvalue_2) (`KismetSystemLibrary.SphereTraceSingleForObjects` :`Start` _returnvalue :`End` _returnvalue :`Radius` 425.0 :`ObjectTypes` (`|MakeArray` "ObjectTypeQuery9" :!type "EObjectTypeQuery Enum") :`DrawDebugType` "ForDuration"))
  (if _returnvalue_2
    (message `/Game/Systems/SimpleDamage/Blueprints/Interfaces/BPI_Damagable.IF_TakeDamage` (`.HitActor` (`GameplayStatics.BreakHitResult` _outhit)) (make `/Game/Systems/SimpleDamage/Blueprints/Data/S_DamageInfo` :`Amount` 5.0)))
  (`GameplayStatics.SpawnEmitterAtLocation` "/Game/Systems/SimpleDamage/FXVarietyPack/Particles/P_ky_explosion.P_ky_explosion" (`self.K2_GetActorLocation`))
  (`GameplayStatics.PlaySoundAtLocation` "/Engine/EditorSounds/GamePreview/PossessPlayer_Cue.PossessPlayer_Cue" (`self.K2_GetActorLocation`) (struct) 1.0 1.0 0.0 null null null null)
  (`self.K2_DestroyActor`))

(fn `UserConstructionScript`)