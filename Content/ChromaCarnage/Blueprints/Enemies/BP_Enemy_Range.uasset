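; Ranged enemy Blueprint that fires a telegraphed hitscan shot at the player.
; IFAttack plays a slowed charge montage while a looping timer re-traces toward the player to stretch a visible Cable as an aim beam.
; The montage notify clears AI focus, hides the beam, re-traces to damage the hit actor, and spawns impact effects and sound.
; Montage completion or interruption signals IFAttackEnd.
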(event `CustomEvent`
  (bind (_outhit _returnvalue) (`KismetSystemLibrary.LineTraceSingleForObjects` (`self.K2_GetActorLocation`) (`self.K2_GetActorLocation` (`GameplayStatics.GetPlayerCharacter` 0)) (`|MakeArray` "ObjectTypeQuery1" "ObjectTypeQuery9" :!type "EObjectTypeQuery Enum")))
  (if _returnvalue
    (set `CableComponent.EndLocation` (`KismetMathLibrary.InverseTransformLocation` (`self.GetTransform`) (`.ImpactPoint` (`GameplayStatics.BreakHitResult` _outhit))) (`self.Cable`))))

(event `self.IF_Attack`
  (params (AttackTarget :type "Actor Object Reference") (IsMeleeAttack :type Boolean))
  (`parent.IF_Attack` AttackTarget false)
  (`SceneComponent.SetVisibility` (`self.Cable`) true false)
  (bind _notifyname (`|PlayMontage` (`self.Mesh`) "/Game/Characters/Mannequins/Anims/Unarmed/Attack/MM_ChargedAttack_Montage.MM_ChargedAttack_Montage" 0.5)
    (:`then`
      (bind _returnvalue (`KismetSystemLibrary.K2_SetTimerDelegate` (delegate `CustomEvent`) 0.25 true))
      (`GameplayStatics.PlaySoundAtLocation` "/Engine/EngineSounds/1kSineTonePing.1kSineTonePing" (`self.K2_GetActorLocation`) (struct) 1.0 1.0 0.0 null null null null))
    (:`OnCompleted`
      (`/Game/Systems/SimpleDamage/Blueprints/Interfaces/BPI_Damagable.IF_AttackEnd` AttackTarget :!label _label))
    (:`OnInterrupted`
      (goto _label))
    (:`OnNotifyBegin`
      (switch `name` _notifyname
        (:`Attack`
          (`AIController.K2_ClearFocus` (`AIBlueprintHelperLibrary.GetAIController` self))
          (`SceneComponent.SetVisibility` (`self.Cable`) false false)
          (`KismetSystemLibrary.K2_ClearAndInvalidateTimerHandle` _returnvalue)
          (bind (_outhit _returnvalue_2) (`KismetSystemLibrary.LineTraceSingleForObjects` (`self.K2_GetActorLocation`) (`self.K2_GetActorLocation` (`GameplayStatics.GetPlayerCharacter` 0)) (`|MakeArray` "ObjectTypeQuery1" "ObjectTypeQuery9" :!type "EObjectTypeQuery Enum")))
          (if _returnvalue_2
            (bind (_bblockinghit _binitialoverlap _time _distance _location _impactpoint _normal _impactnormal _physmat _hitactor) (`GameplayStatics.BreakHitResult` _outhit))
            (message `/Game/Systems/SimpleDamage/Blueprints/Interfaces/BPI_Damagable.IF_TakeDamage` _hitactor (make `/Game/Systems/SimpleDamage/Blueprints/Data/S_DamageInfo` :`Amount` 5.0)))
          (`GameplayStatics.SpawnEmitterAtLocation` "/Game/Systems/SimpleDamage/FXVarietyPack/Particles/P_ky_hit1.P_ky_hit1" _location)
          (`GameplayStatics.PlaySoundAtLocation` "/Engine/VREditor/Sounds/UI/Camera_Shutter.Camera_Shutter" (`self.K2_GetActorLocation`) (struct) 1.0 1.0 0.0 null null null null))))))

(fn `UserConstructionScript`
  (`parent.UserConstructionScript`))