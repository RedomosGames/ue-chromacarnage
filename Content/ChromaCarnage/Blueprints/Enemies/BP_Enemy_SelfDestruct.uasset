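; BP_Enemy_SelfDestruct is an enemy Blueprint whose attack destroys the enemy itself.
; On IFAttack it runs the parent attack logic, then plays the MM_Land montage on its mesh.
; Whether the montage completes or is interrupted, it signals IFAttackEnd, spawns an explosion emitter at its location and destroys the actor one tick later.
; No damage is applied in this graph, and BeginPlay is disabled.
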(event `self.IF_Attack`
  (params (AttackTarget :type "Actor Object Reference"))
  (`parent.IF_Attack` AttackTarget)
  (`|PlayMontage` (`self.Mesh`) "/Game/Characters/Mannequins/Anims/Unarmed/Jump/MM_Land_Montage.MM_Land_Montage"
    (:`OnCompleted`
      _)
    (:`OnInterrupted`
      _))
  (`/Game/Systems/SimpleDamage/Blueprints/Interfaces/BPI_Damagable.IF_AttackEnd` AttackTarget)
  (`GameplayStatics.SpawnEmitterAtLocation` "/Game/Systems/SimpleDamage/FXVarietyPack/Particles/P_ky_explosion.P_ky_explosion" (`self.K2_GetActorLocation`))
  (`KismetSystemLibrary.DelayUntilNextTick`)
  (`self.K2_DestroyActor`))

(fn `UserConstructionScript`
  (`parent.UserConstructionScript`))