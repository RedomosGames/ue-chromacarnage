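; BP_LootRoom is a dungeon loot room that awards the player a random weapon.
; Its CELootRoom override runs the parent logic, then rolls one of five weapons and adds the matching gameplay tag to the player's weapon info container.
; The same index sets the displayed weapon mesh and is passed to the player's CEShowLootRoomWeapon, with an explosion effect spawned just below the mesh.
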(event `self.ReceiveBeginPlay`
  (`parent.ReceiveBeginPlay`))

(event `self.CE_LootRoom`
  (bind _weaponmesh (`self.WeaponMesh`))
  (bind _randomweaponint (`self.RandomWeaponInt`))
  (bind (_returnvalue_x _returnvalue_y _returnvalue_z) (`KismetMathLibrary.BreakVector` (`SceneComponent.K2_GetComponentLocation` _weaponmesh)))
  (`parent.CE_LootRoom`)
  (set `self.RandomWeaponInt` (`KismetMathLibrary.RandomIntegerInRange` 0 4))
  (`BlueprintGameplayTagLibrary.AddGameplayTag` (`.PlayerWeaponInfoContainer_49_7BE4CF1948EE88B72CFC08B1D3DEC64E` (break `/Game/Systems/Guns/Blueprints/Data/Structs/S_GunPlayerInfo` (`/Game/ChromaCarnage/Default/BP_Player.GunPlayerInfo` (`self.PlayerRef`)))) (select `int` _randomweaponint :`0` (struct :`TagName` "Gun.Weapons.Corroder") :`1` (struct :`TagName` "Gun.Weapons.CrimsonHelix") :`2` (struct :`TagName` "Gun.Weapons.Eclipser") :`3` (struct :`TagName` "Gun.Weapons.GlacierBeam") :`4` (struct :`TagName` "Gun.Weapons.ThunderJaw") :!type "GameplayTag Structure"))
  (`StaticMeshComponent.SetStaticMesh` _weaponmesh (select `int` _randomweaponint :`0` "/Game/Imports/Models/aAuto.aAuto" :`1` "/Game/Imports/Models/aSemi.aSemi" :`2` "/Game/Imports/Models/aBeam.aBeam" :`3` "/Game/Imports/Models/aBurst.aBurst" :`4` "/Game/Imports/Models/aShotgun.aShotgun" :!type "StaticMesh Object Reference"))
  (`NiagaraFunctionLibrary.SpawnSystemAtLocation` "/Game/LowPolyVFX/Particles/P_Explosion_01_Converted.P_Explosion_01_Converted" (`KismetMathLibrary.MakeVector` _returnvalue_x _returnvalue_y (+ _returnvalue_z -50.0)) (struct) (5.0 5.0 5.0))
  (`/Game/ChromaCarnage/Default/BP_Player.CE_ShowLootRoomWeapon` (`self.PlayerRef`) (`self.RandomWeaponInt`)))

(fn `UserConstructionScript`
  (`parent.UserConstructionScript`))