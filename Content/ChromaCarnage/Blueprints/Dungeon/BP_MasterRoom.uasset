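; Master dungeon room actor that reacts the first time the player enters, based on its room type.
; On actor overlap, box components under RoomDetection check for the player, and a flag blocks repeat triggers.
; Combat and Boss rooms notify GS_Game; Combat then waits briefly, sets the enemy count and spawns random enemy types at random floor points, removing each used point.
; Spawn rooms only print, and Loot is an empty stub.
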(event `self.ReceiveBeginPlay`
  ;[0 1 1 0.5] Begin Play
  (add `self.OnActorBeginOverlap` (`|CreateDelegate` :!event `B_ActorBeginOverlap`))
  (bind _asgs_game (cast `/Game/ChromaCarnage/Default/GS_Game` (`GameplayStatics.GetGameState`)))
  (set `self.GS` _asgs_game)
  (`self.CE_AddFloorSpawnPointsToList`)
  (bind _asbp_player (cast `/Game/ChromaCarnage/Default/BP_Player` (`GameplayStatics.GetPlayerCharacter` 0)))
  (set `self.PlayerRef` _asbp_player))

(event `CE_CombatRoom`
  (`/Game/ChromaCarnage/Default/GS_Game.OnPlayerEnteredRoom` (`self.GS`))
  (`KismetSystemLibrary.Delay` 1.0)
  (`self.CE_SpawnEnemiesInRoom` true 10 (0.0 0.0 100.0)))

(event `B_ActorBeginOverlap` :!signature `self.OnActorBeginOverlap`
  (params (OverlappedActor :type "Actor Object Reference") (OtherActor :type "Actor Object Reference"))
  ;[0 1 0 0.5] Detect Overlap in Room / Determine if player has been hrere already
  (for _array_element (`SceneComponent.GetChildrenComponents` (`self.RoomDetection`) false)
    (bind _asbox_collision (cast `BoxComponent` _array_element))
    (for _ (`PrimitiveComponent.GetOverlappingActors` _asbox_collision "/Game/ChromaCarnage/Default/BP_Player.BP_Player_C")
      (if (not (`self.HasEntered`))
        (`KismetSystemLibrary.PrintString` "Entered")
        (set `self.HasEntered` true)
        (switch `/Game/ChromaCarnage/Blueprints/Dungeon/E_RoomType` (`self.RoomType`)
          (:`NewEnumerator0`
            (`KismetSystemLibrary.PrintString` "Select A Room"))
          (:`NewEnumerator1`
            (`KismetSystemLibrary.PrintString` "Spawn Room"))
          (:`NewEnumerator2`
            (`self.CE_CombatRoom`))
          (:`NewEnumerator3`
            (`self.CE_LootRoom`))
          (:`NewEnumerator4`
            (`self.CE_BossRoom`)))
        (else
          (`KismetSystemLibrary.PrintString` "Already Entered"))))))

(event `CE_LootRoom`)

(event `CE_BossRoom`
  (`/Game/ChromaCarnage/Default/GS_Game.OnPlayerEnteredRoom` (`self.GS`)))

(event `CE_AddFloorSpawnPointsToList`
  ;[0 1 0 0.5] Get Enemy Spawn Positions
  (`KismetArrayLibrary.Array_Append` (`self.FloorSpawnList`) (`SceneComponent.GetChildrenComponents` (`self.FloorSpawnPointsFolder`) false)))

(event `CE_SpawnEnemiesInRoom`
  (params (`ShouldSpawnItem?` :type Boolean) (ItemSpawnAmount :type Integer) (SpawnOffset :type "Vector Structure"))
  ;[0 1 0 0.5] Find Spawn Location and Spawn Enemy
  (if `ShouldSpawnItem?`
    (set `/Game/ChromaCarnage/Default/GS_Game.EnemySpawnCount` ItemSpawnAmount (`self.GS`))
    (if (> ItemSpawnAmount 0) :!label _label
      (set `self.SelectedFloorSpawnLocation` (`KismetArrayLibrary.Array_Random` (`self.FloorSpawnList`)))
      (`|SpawnActorFromClass` (`KismetArrayLibrary.Array_Random` (`self.EnemyTypes`)) (`KismetMathLibrary.MakeTransform` (+ (`SceneComponent.K2_GetComponentLocation` (`self.SelectedFloorSpawnLocation`)) SpawnOffset)) "AlwaysSpawn" "MultiplyWithRoot" null null)
      (`KismetArrayLibrary.Array_RemoveItem` (`self.FloorSpawnList`) (`self.SelectedFloorSpawnLocation`))
      (`|VariableSetRef` ItemSpawnAmount (- ItemSpawnAmount 1))
      (goto _label))))

(fn `UserConstructionScript`)