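; Procedural dungeon generator that grows a level from a start room by attaching random rooms to open exits, using a seedable random stream.
; Overlapping rooms are destroyed and retried; accepted rooms add exits, with special rooms at set counts and a boss room last.
; On completion it caps holes, spawns doors and notifies the game state.
; A watchdog timer reloads the level if game time exceeds the limit during generation.
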(event `self.ReceiveBeginPlay`
  ;[0 1 1 0.5] Begin Play / Check Seed / Spawn Start Room / Start Timer / Spawn Next Room
  (`self.CE_SetSeed`)
  (`self.CE_SpawnStartRoom`)
  (`self.CE_StartDungeonTimer`)
  (`self.CE_SpawnNextRoom`)
  (bind _asgs_game (cast `/Game/ChromaCarnage/Default/GS_Game` (`GameplayStatics.GetGameState`)))
  (set `self.GS` _asgs_game))

(event `CE_SpawnStartRoom`
  ;[0 1 0 0.5] CE_SpawnStartRoom / Spawn the room the player starts in
  ;;[1 1 0 0.5] Set Spawn Room here
  (bind _returnvalue (`|SpawnActorFromClass` "/Game/ChromaCarnage/Blueprints/Dungeon/BP_SpawnRoom.BP_SpawnRoom_C" (`SceneComponent.K2_GetComponentToWorld` (`self.DefaultSceneRoot`)) "AlwaysSpawn" "MultiplyWithRoot" null null))
  (`KismetArrayLibrary.Array_Append` (`self.ExitsList`) (`SceneComponent.GetChildrenComponents` (`/Game/ChromaCarnage/Blueprints/Dungeon/BP_MasterRoom.ExitsFolder` _returnvalue) false))
  (set `self.SpawnRoomList` (`self.BaseRoomList`)))

(event `CE_SpawnNextRoom`
  ;[0 1 0 0.5] CE_SpawnNextRoom / Get a room from 'RoomList' and spawn that room at an exit as long as 'RoomAmount' has spawns left
  (bind _output_get (set `self.SelectedExitPoint` (`KismetArrayLibrary.Array_RandomFromStream` (`self.ExitsList`) (`self.Stream`))))
  (bind _returnvalue (`|SpawnActorFromClass` (`KismetArrayLibrary.Array_RandomFromStream` (`self.SpawnRoomList`) (`self.Stream`)) (`SceneComponent.K2_GetComponentToWorld` _output_get) "AlwaysSpawn" "MultiplyWithRoot" null null))
  (bind _asbp_master_room (cast `/Game/ChromaCarnage/Blueprints/Dungeon/BP_MasterRoom` _returnvalue))
  (set `self.LatestRoom` _asbp_master_room)
  (`KismetSystemLibrary.DelayUntilNextTick`)
  (`self.CE_CheckForOverlap`))

(event `CE_AddOverlappingRoomsToList`
  ;[0 1 0 0.5] CE_AddOverlappingRoomsToList / If room spawns on top of other room, add to list
  (for _array_element (`SceneComponent.GetChildrenComponents` (`/Game/ChromaCarnage/Blueprints/Dungeon/BP_MasterRoom.OverlapFolder` (`self.LatestRoom`)) false)
    (bind _asbox_collision (cast `BoxComponent` _array_element))
    (`KismetArrayLibrary.Array_Append` (`self.OverlappedList`) (`PrimitiveComponent.GetOverlappingComponents` _asbox_collision))))

(event `CE_CheckForOverlap`
  ;[0 1 0 0.5] CE_CheckForOverlap / Check if dungeon room spawned on top of other room, is so, destroy itself an respawn
  (`self.CE_AddOverlappingRoomsToList`)
  (if (`KismetArrayLibrary.Array_IsNotEmpty` (`self.OverlappedList`))
    (`KismetArrayLibrary.Array_Clear` (`self.OverlappedList`))
    (`self.K2_DestroyActor` (`self.LatestRoom`))
    (`self.CE_SpawnNextRoom`)
    (else
      (`KismetArrayLibrary.Array_Clear` (`self.OverlappedList`))
      (set `self.RoomAmount` (- (`self.RoomAmount`) 1))
      (`KismetArrayLibrary.Array_RemoveItem` (`self.ExitsList`) (`self.SelectedExitPoint`))
      (`KismetArrayLibrary.Array_Add` (`self.DoorList`) (`self.SelectedExitPoint`))
      (if (`self.IsLinear?`)
        (`KismetArrayLibrary.Array_Clear` (`self.ExitsList`)))
      (`KismetArrayLibrary.Array_Append` (`self.ExitsList`) (`SceneComponent.GetChildrenComponents` (`/Game/ChromaCarnage/Blueprints/Dungeon/BP_MasterRoom.ExitsFolder` (`self.LatestRoom`)) false))
      (`self.CE_AddFloorSpawnPointsToList`)
      (if (> (`self.RoomAmount`) 0)
        (`self.F_ChooseSpawnType`)
        (else
          (`self.CE_CloseHoles`)
          (`self.CE_SpawnDoors`)
          (set `self.DungeonComplete?` true)
          (`KismetSystemLibrary.K2_ClearAndInvalidateTimerHandle` (`self.StartDungeonTimerHandle`))
          (`KismetSystemLibrary.PrintString` "Dungeon Compelte" true true (struct :`R` 1.0 :`G` 0.843763 :`B` 0.32103 :`A` 1.0) 10.0)
          (`KismetSystemLibrary.DelayUntilNextTick`)
          (`/Game/ChromaCarnage/Default/GS_Game.OnDungeonGenerationComplete` (`self.GS`)))))))

(event `CE_CloseHoles`
  ;[0 1 0 0.5] CE_CloseHoles / When Dungeon Generated, Close all open holes
  (for _array_element (`self.ExitsList`)
    (`|SpawnActorFromClass` (`self.CloseHole`) (`SceneComponent.K2_GetComponentToWorld` _array_element) "AlwaysSpawn" "MultiplyWithRoot" null null)))

(event `CE_AddFloorSpawnPointsToList`
  ;[0 1 0 0.5] CE_AddFloorSpawnPointsToList / Add Floor Spawn Points to Array
  (`KismetArrayLibrary.Array_Append` (`self.FloorSpawnList`) (`SceneComponent.GetChildrenComponents` (`/Game/ChromaCarnage/Blueprints/Dungeon/BP_MasterRoom.FloorSpawnPointsFolder` (`self.LatestRoom`)) false)))

(event `CE_StartDungeonTimer`
  ;[0 1 0 0.5] CE_StartDungeonTimer / Check how long has passed while creating dungeon, reset if to long
  (bind _returnvalue (`KismetSystemLibrary.K2_SetTimerDelegate` (delegate `StartDungeonTimer`) 1.0 true))
  (set `self.StartDungeonTimerHandle` _returnvalue))

(event `CE_SpawnItemAtLocation`
  (params (`ShouldSpawnItem?` :type Boolean) (ItemSpawnAmount :type Integer) (ItemSpawnClass :type "Actor Class Reference") (SpawnOffset :type "Vector Structure"))
  ;[0 1 0 0.5] CE_SpawnItemAtLocation / Take Inputs and Spawn Actor at random Location
  (if `ShouldSpawnItem?`
    (if (> ItemSpawnAmount 0) :!label _label
      (set `self.SelectedFloorSpawnLocation` (`KismetArrayLibrary.Array_RandomFromStream` (`self.FloorSpawnList`) (`self.Stream`)))
      (`|SpawnActorFromClass` ItemSpawnClass (`KismetMathLibrary.MakeTransform` (+ (`SceneComponent.K2_GetComponentLocation` (`self.SelectedFloorSpawnLocation`)) SpawnOffset)) "AlwaysSpawn" "MultiplyWithRoot" null null)
      (`KismetArrayLibrary.Array_RemoveItem` (`self.FloorSpawnList`) (`self.SelectedFloorSpawnLocation`))
      (`|VariableSetRef` ItemSpawnAmount (- ItemSpawnAmount 1))
      (goto _label))))

(event `StartDungeonTimer`
  ;[0 1 0 0.5] CE_StartDungeonTimer / Check how long has passed while creating dungeon, reset if to long
  (if (>= (`KismetSystemLibrary.GetGameTimeInSeconds`) (`self.MaxDungeonSpawnTime`))
    (`GameplayStatics.OpenLevelBySoftObjectPtr` "/Game/Systems/ProceduralDungeon/Default/LVL_ProceduralDungeon.LVL_ProceduralDungeon")))

(event `CE_SetSeed`
  (bind _stream (`self.Stream`))
  ;[0 1 0 0.5] CE_SetSeed / Check Seed input for a random dungeon or a seed dungeon
  (if (== (`self.Seed`) -1)
    (`KismetMathLibrary.SeedRandomStream` (`self.Stream`))
    (else
      (`KismetMathLibrary.SetRandomStreamSeed` _stream (`self.Seed`))))
  (`KismetSystemLibrary.PrintString` (`KismetStringLibrary.Conv_IntToString` (`KismetMathLibrary.BreakRandomStream` _stream)) true true (struct :`R` 1.0 :`B` 0.787341 :`A` 1.0) 30.0))

(event `CE_SpawnDoors`
  ;[0 1 0 0.5] CE_SpawnDoors / Spawn a door where rooms connect
  (for _array_element (`self.DoorList`)
    (`|SpawnActorFromClass` (`KismetArrayLibrary.Array_RandomFromStream` (`self.DoorActor`) (`self.Stream`)) (`SceneComponent.K2_GetComponentToWorld` _array_element) "AlwaysSpawn" "MultiplyWithRoot" null null)))

(fn `F_CheckSpecialRoomSpawn`
  (returns (`SpawnSpecialRoom?` :type Boolean))
  (locals (`GotNumber?` :type Boolean))
  (for _array_element (`self.SpecialRoomNumber`)
    (if (== (`self.RoomAmount`) _array_element)
      (set `local.GotNumber?` true)))
  (if (`local.GotNumber?`)
    (set `local.GotNumber?` false)
    (return true)
    (else
      (set `local.GotNumber?` false)
      (return false))))

(fn `F_ChooseSpawnType`
  (if (== (`self.RoomAmount`) 1)
    (set `self.SpawnRoomList` (`self.BossRoomList`))
    (`KismetSystemLibrary.PrintString` "Boss" true true (struct :`R` 1.0 :`A` 1.0))
    (`self.CE_SpawnNextRoom`)
    (else
      (bind _spawnspecialroom_ (`self.F_CheckSpecialRoomSpawn`))
      (if _spawnspecialroom_
        (set `self.SpawnRoomList` (`self.SpecialRoomList`))
        (`KismetSystemLibrary.PrintString` "Special" true true (struct :`R` 0.443478 :`B` 1.0 :`A` 1.0))
        (else
          (set `self.SpawnRoomList` (`self.BaseRoomList`))
          (`KismetSystemLibrary.PrintString` "Base")))
      (`self.CE_SpawnNextRoom`))))

(fn `UserConstructionScript`)