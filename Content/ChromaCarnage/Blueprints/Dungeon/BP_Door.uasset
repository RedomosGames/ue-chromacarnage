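; BP_Door is a two-panel sliding dungeon door that closes when the player enters a room and opens when the room is cleared.
; One tick after BeginPlay it binds to the room-entered and room-cleared dispatchers on GS_Game.
; Two timelines lerp the left and right panels along relative Y in opposite directions, playing forward to open and reversing to close.
; The handlers do not check which room fired the event.
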(event `self.ReceiveBeginPlay`
  ;[0 1 0 0.5] Begin Play
  (`KismetSystemLibrary.DelayUntilNextTick`)
  (bind _asgs_game (cast `/Game/ChromaCarnage/Default/GS_Game` (`GameplayStatics.GetGameState`)))
  (add `/Game/ChromaCarnage/Default/GS_Game.OnPlayerEnteredRoom` _asgs_game (`|CreateDelegate` :!event `B_OnPlayerEnteredRoom`))
  (add `/Game/ChromaCarnage/Default/GS_Game.OnPlayerClearedRoom` _asgs_game (`|CreateDelegate` :!event `B_OnPlayerClearedRoom`)))

(event `B_OnPlayerClearedRoom`
  (bind _rightdoor (`self.RightDoor`))
  (bind _leftdoor (`self.LeftDoor`))
  (bind (_relativelocation_x _relativelocation_y _relativelocation_z) (`KismetMathLibrary.BreakVector` (`SceneComponent.RelativeLocation` _rightdoor)))
  (bind (_relativelocation_x_2 _relativelocation_y_2 _relativelocation_z_2) (`KismetMathLibrary.BreakVector` (`SceneComponent.RelativeLocation` _leftdoor)))
  (`|ExecutionSequence`
    (:`then_0`
      (bind (_direction _newtrack_0) (`Timeline|Timeline` :!label _label)
        (:`Update`
          (`SceneComponent.K2_SetRelativeLocation` _leftdoor (`KismetMathLibrary.MakeVector` _relativelocation_x_2 (`KismetMathLibrary.Lerp` 125.0 325.0 _newtrack_0) _relativelocation_z_2) false false))))
    (:`then_1`
      (bind (_direction_2 _newtrack_0_2) (`Timeline|Timeline_0` :!label _label_2)
        (:`Update`
          (`SceneComponent.K2_SetRelativeLocation` _rightdoor (`KismetMathLibrary.MakeVector` _relativelocation_x (`KismetMathLibrary.Lerp` -125.0 -325.0 _newtrack_0_2) _relativelocation_z) false false))))))

(event `B_OnPlayerEnteredRoom`
  (`|ExecutionSequence`
    (:`then_0`
      (goto _label :!via `Reverse`))
    (:`then_1`
      (goto _label_2 :!via `Reverse`))))

(fn `UserConstructionScript`)